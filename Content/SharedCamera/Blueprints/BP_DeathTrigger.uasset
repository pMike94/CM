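; BP_DeathTrigger is a box volume that kills pawns entering it in a shared-camera game.
; It finds the first BP_Camera at BeginPlay, then on overlap destroys any Pawn and calls that camera's CameraToPlayerReset.
; The construction script sizes the box from the BoxSize variable.
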(event OnComponentBeginOverlap(DeathTrigger)
  (params (OverlappedComponent :type Primitive%20Component%20Object%20Reference) (OtherActor :type Actor%20Object%20Reference) (OtherComp :type Primitive%20Component%20Object%20Reference) (OtherBodyIndex :type Integer) (bFromSweep :type Boolean) (SweepResult :type Hit%20Result%20Structure%20%28by%20ref%29))
  (bind _aspawn (Utilities|Casting|CastToPawn OtherActor))
  (Actor|DestroyActor _aspawn)
  (Default|CameratoPlayerReset (Variables|Default|GetCamera)))

(event EventBeginPlay
  (bind _outactors (Actor|GetAllActorsOfClass "/Game/SharedCamera/Blueprints/Camera/BP_Camera.BP_Camera_C"))
  (Variables|Default|SetCamera (Utilities|Array|Get(acopy) _outactors)))

(fn ConstructionScript
  (Components|Box|SetBoxExtent (Variables|Default|GetDeathTrigger) (Variables|Default|GetBoxSize) true))