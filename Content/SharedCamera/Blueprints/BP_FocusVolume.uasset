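; BP_FocusVolume is a box trigger that shifts the shared BP_Camera's focus from the players to a fixed Focus point.
; When overlapping pawns reach PlayersNeeded, it stops the camera's UpdateCam timer, transitions to Focus, then applies max zoom after a delay.
; A pawn exiting at that count calls CameraToPlayerReset; the counter only decrements then.
; The construction script applies box size and focus location.
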(event OnComponentBeginOverlap(Box)
  (params (OverlappedComponent :type Primitive%20Component%20Object%20Reference) (OtherActor :type Actor%20Object%20Reference) (OtherComp :type Primitive%20Component%20Object%20Reference) (OtherBodyIndex :type Integer) (bFromSweep :type Boolean) (SweepResult :type Hit%20Result%20Structure%20%28by%20ref%29))
  ;[1 0.5769 0] Add a Player to the Box
  (Utilities|Casting|CastToPawn OtherActor)
  (Variables|Default|SetPlayersInBox (+ (Variables|Default|GetPlayersInBox) 1))
  (CallFunction|OnFocusChange))

(event OnComponentEndOverlap(Box)
  (params (OverlappedComponent :type Primitive%20Component%20Object%20Reference) (OtherActor :type Actor%20Object%20Reference) (OtherComp :type Primitive%20Component%20Object%20Reference) (OtherBodyIndex :type Integer))
  ;[1 0.8603 0] Check if Players in Box Equal to Players needed
  (Utilities|Casting|CastToPawn OtherActor)
  (if (== (Variables|Default|GetPlayersInBox) (Variables|Default|GetPlayersNeeded))
    (CallFunction|OnFocusPlayer)))

(event Custom|OnFocusChange
  (bind _camera (Variables|Default|GetCamera))
  (bind _camera_2 (Variables|Default|GetCamera))
  (bind _focus (Variables|Default|GetFocus))
  (bind _returnvalue (Transformation|GetWorldLocation _focus))
  ;[1 0.9458 0] Check if Players in Box equal to Players Needed
  (if (== (Variables|Default|GetPlayersInBox) (Variables|Default|GetPlayersNeeded))
    (Utilities|Time|ClearTimerbyFunctionName (Variables|Default|GetCamera) "UpdateCam")
    ;[0 0.4365 1] Set the Focus on the Focusable Object
    (Variables|/Game/SharedCamera/Blueprints/Camera/BP_Camera.BP_Camera_C|SetTargetLoc (Variables|Default|GetCamera) _returnvalue)
    (Default|OnTransition _camera)
    (Utilities|FlowControl|Delay (* 1.0 (Variables|/Game/SharedCamera/Blueprints/Camera/BP_Camera.BP_Camera_C|GetResetTransitionSpeed _camera)))
    (Variables|/Game/SharedCamera/Blueprints/Camera/BP_Camera.BP_Camera_C|SetCurrentLoc _camera_2 _returnvalue)
    (Variables|/Game/SharedCamera/Blueprints/Camera/BP_Camera.BP_Camera_C|SetCurrentZoom _camera_2 (Variables|/Game/SharedCamera/Blueprints/Camera/BP_Camera.BP_Camera_C|GetMaxDistance _camera_2))))

(event Custom|OnFocusPlayer
  ;[0 0.7169 1] Set the Focus back to the Player
  (Variables|Default|SetPlayersInBox (- (Variables|Default|GetPlayersInBox) 1))
  (Default|CameratoPlayerReset (Variables|Default|GetCamera)))

(event EventBeginPlay
  (bind _outactors (Actor|GetAllActorsOfClass "/Game/SharedCamera/Blueprints/Camera/BP_Camera.BP_Camera_C"))
  (Variables|Default|SetCamera (Utilities|Array|Get(acopy) _outactors)))

(fn ConstructionScript
  (Components|Box|SetBoxExtent (Variables|Default|GetBox) (Variables|Default|GetBoxSize) true)
  (Transformation|SetRelativeLocation (Variables|Default|GetFocus) (Variables|Default|GetFocusLocation) false false))