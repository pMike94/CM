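; Shared multiplayer camera that frames all Character actors and becomes the player controllers' view target.
; A looping timer moves it to their average position plus offset, with optional axis locks, and sets spring arm length from the largest pairwise distance, clamped to zoom limits.
; CameraToPlayerReset pauses that timer, re-gathers players and blends position and zoom through a timeline with configurable curves and speed, then resumes updates.
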(event Custom|UpdateCam
  (CallFunction|TargerArmUpdate)
  (Variables|Zoom|SetCurrentZoom (Variables|Zoom|GetMaxDistance))
  (CallFunction|LocationUpdate)
  ;[1 0 0] Reset fMaxDistance for the nex call of the Function
  (Variables|Zoom|SetMaxDistance 0.0))

(event Custom|OnTransition
  (bind (_direction _alphapos _alphazoom) (Timeline|TL_Postion PlayFromStart)
    (:Update
      (Transformation|SetActorLocation (Math|Vector|Lerp(Vector) (Variables|Location|GetCurrentLoc) (Variables|Location|GetTargetLoc) _alphapos) true true)
      (Variables|/Script/Engine.SpringArmComponent|SetTargetArmLength (Variables|Components|GetSpringArm) (Math|Float|Clamp(Float) (Math|Float|Lerp (Variables|Zoom|GetCurrentZoom) (Variables|Zoom|GetMaxDistance) _alphazoom) (Variables|Zoom|GetMinCamaraZoom) (Variables|Zoom|GetMaxCameraZoom))))
    (:Finished
      ;[1 0 0] Start fUpdateCam after Death Fade
      (Utilities|Time|SetTimerbyFunctionName 0 "UpdateCam" (Variables|Default|GetCamUpdateInterval) true))))

(event Custom|CameraToPlayerReset
  (CallFunction|SetPlayersArray)
  (CallFunction|SetTargetLocation)
  (CallFunction|SetMaxDistance)
  (Variables|Zoom|SetTargetZoom (Variables|Zoom|GetMaxDistance))
  (CallFunction|OnTransition))

(event EventBeginPlay
  (CallFunction|TimelineInitSettings)
  (CallFunction|Debug)
  (Utilities|FlowControl|Delay 0.2)
  (CallFunction|SetPlayersArray)
  (Utilities|Time|SetTimerbyFunctionName 0 "UpdateCam" (Variables|Default|GetCamUpdateInterval) true))

(fn ConstructionScript
  ;[0 0.1805 1] Set Rotation
  (Transformation|SetRelativeRotation (Variables|Components|GetSpringArm) "0, 0, 0" false false))

(fn TargerArmUpdate
  (CallFunction|SetMaxDistance)
  ;[0 0.1736 1] Set Arm Length of the Spring Arm (Zoom)
  (Variables|/Script/Engine.SpringArmComponent|SetTargetArmLength (Variables|Components|GetSpringArm) (Math|Float|Clamp(Float) (Variables|Zoom|GetMaxDistance) (Variables|Zoom|GetMinCamaraZoom) (Variables|Zoom|GetMaxCameraZoom))))

(fn LocationUpdate
  (CallFunction|SetTargetLocation)
  (Transformation|SetActorLocation (Variables|Location|GetTargetLoc) false false)
  (Variables|Location|SetCurrentLoc (Transformation|GetActorLocation))
  ;[1 0.01736 0] Reset "vAddedLOC"
  (Variables|Location|SetAddedLOC "0, 0, 0"))

(fn Debug
  ;[0 0.1911 1] Set Debug Cube Visible in Game
  (if (Variables|Default|GetDebugging)
    (Development|SetHiddeninGame (Variables|Components|GetDebugCube) false false)))

(fn LockAxis
  ;[0 0.2309 1] Lock X Axis at wished position
  (if (Variables|Location|GetLockX)
    (Variables|Location|SetTargetLoc (Math|Vector|MakeVector (Variables|Location|GetLockXPos) (.y (Variables|Location|GetTargetLoc)) (.z (Variables|Location|GetTargetLoc)))))
  ;[0 0.3115 1] Lock Y Axis at wished Position
  (if (Variables|Location|GetLockY)
    (Variables|Location|SetTargetLoc (Math|Vector|MakeVector (.x (Variables|Location|GetTargetLoc)) (Variables|Location|GetLockYPos) (.z (Variables|Location|GetTargetLoc)))))
  ;[0 0.3375 1] Lock Z Axis at wished Postion
  (if (Variables|Location|GetLockZ)
    (Variables|Location|SetTargetLoc (Math|Vector|MakeVector (.x (Variables|Location|GetTargetLoc)) (.y (Variables|Location|GetTargetLoc)) (Variables|Location|GetLockZPos)))))

(fn SetTargetLocation
  ;[1 0.8016 0] Add all Player locations to one vector
  (for _array_element (Variables|Default|GetPlayers)
    (Variables|Location|SetAddedLOC (+ (Transformation|GetActorLocation _array_element) (Variables|Location|GetAddedLOC))))
  ;[0 0.1509 1] Set camera Location to the MidLocation of the Players
  (Variables|Location|SetTargetLoc (+ (/ (Variables|Location|GetAddedLOC) (Utilities|Array|Length (Variables|Default|GetPlayers))) (Variables|Location|GetCameraOffset)))
  (CallFunction|LockAxis))

(fn SetMaxDistance
  ;[1 0.7573 0] Check which players have the furthest Distance to each other
  (for _array_element (Variables|Default|GetPlayers)
    (for _array_element_2 (Variables|Default|GetPlayers)
      (if (> (Transformation|GetDistanceTo _array_element _array_element_2) (Variables|Zoom|GetMaxDistance))
        (Variables|Zoom|SetMaxDistance (Transformation|GetDistanceTo _array_element _array_element_2))))))

(fn TimelineInitSettings
  ;[0 0.2825 1] Set Movement Curves for Camera onPlayerReset
  (Class|TimelineComponent|SetFloatCurve (Variables|Default|GetTL_Postion) (Variables|Death|GetDeathChangePositionCurve) "AlphaPOS")
  (Class|TimelineComponent|SetFloatCurve (Variables|Default|GetTL_Postion) (Variables|Death|GetDeathChangeZoomCurve) "AlphaZoom")
  ;[0 0.3366 1] Set Timeline Speed for onPlayerReset
  (Components|Timeline|SetPlayRate (Variables|Default|GetTL_Postion) (/ 1.0 (Variables|Death|GetDeathChangeSpeed))))

(fn SetPlayersArray
  ;[0.4167 0.01075 0] Reset fUpdateCam on Player Reset
  (Utilities|Time|ClearTimerbyFunctionName 0 "UpdateCam")
  ;[1 0.9052 0] Add Players to the "Players" Array
  (Utilities|Array|Clear (Variables|Default|GetPlayers))
  (bind _outactors (Actor|GetAllActorsOfClass (Variables|Default|GetCharacter)))
  (for _array_element _outactors
    (Utilities|Array|Add (Variables|Default|GetPlayers) _array_element))
  (Variables|Zoom|SetMaxDistance 0.0)
  ;[0 0.2214 1] Set the Controllers as Target for the Camera
  (bind _outactors_2 (Actor|GetAllActorsOfClass (Variables|Default|GetPlayerControllerClass)))
  (Game|Player|SetViewTargetwithBlend _outactors_2 self 0.0 "VTBlend_Linear" 0.0 false))